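; Zombie enemy Blueprint that handles melee damage through the overlap of its Weapon component.
; WeaponActive and WeaponDeactive events switch the weapon's collision between overlapping everything and none.
; On overlap, it applies Damage to actors that are neither Enemy-class nor its owner, with a DoOnce and half-second delay throttling repeat hits.
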(event `self.Weapon.OnComponentBeginOverlap`
  (params (OverlappedComponent :type "PrimitiveComponent Object Reference") (OtherActor :type "Actor Object Reference") (OtherComp :type "PrimitiveComponent Object Reference") (OtherBodyIndex :type Integer) (bFromSweep :type Boolean) (SweepResult :type "HitResult Structure (by ref)"))
  (cast `/Game/enemy/ClassLogic/Enemy` OtherActor
    (:`CastFailed`
      (if (!= OtherActor (`self.GetOwner`))
        (`/Engine/EditorBlueprintResources/StandardMacros.DoOnce` false :!label _label
          (:`Completed`
            (`GameplayStatics.ApplyDamage` OtherActor (`self.Damage`))
            (`KismetSystemLibrary.Delay` 0.5)
            (goto _label :!via `Reset`)))))))

(event `WeaponActive`
  (`PrimitiveComponent.SetCollisionProfileName` (`self.Weapon`) "OverlapAll" true))

(event `WeaponDeactive`
  (`PrimitiveComponent.SetCollisionEnabled` (`self.Weapon`) "NoCollision"))

(fn `UserConstructionScript`
  (`parent.UserConstructionScript`))